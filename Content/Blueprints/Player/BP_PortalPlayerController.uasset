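; Player controller that handles input for creating and destroying the player's pair of portals in a networked game.
; Portal A and B inputs send gameplay events, leaving placement to whatever listens for those tags.
; Destroy inputs scan all BP_Portal actors, using IsExitPortal to tell B from A and a locally controlled Instigator to match ownership.
; Matches are destroyed directly with authority, or through ServerDestroyPortal on clients.
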(event `self.ReceiveBeginPlay`
  (`parent.ReceiveBeginPlay`))

(event `ServerDestroyPortal`
  (params (PortalToDestroy :type "/PortalGame/Blueprints/Portal/BP_Portal Object Reference"))
  (`self.K2_DestroyActor` PortalToDestroy))

(event `EnhancedInput|/PortalGame/Input/Actions/IA_PortalA`
  (params (ActionValue :type Boolean) (ElapsedSeconds :type "Float (double-precision)") (TriggeredSeconds :type "Float (double-precision)") (InputAction :type "InputAction Object Reference" :default "/PortalGame/Input/Actions/IA_PortalA.IA_PortalA"))
  ;[0 0.8583 1] PortalA
  (:`Triggered`
    (`self.SendGameplayEventWithPayload` (struct :`TagName` "Event.PortalA"))))

(event `EnhancedInput|/PortalGame/Input/Actions/IA_DestroyPortalA`
  (params (ActionValue :type Boolean) (ElapsedSeconds :type "Float (double-precision)") (TriggeredSeconds :type "Float (double-precision)") (InputAction :type "InputAction Object Reference" :default "/PortalGame/Input/Actions/IA_DestroyPortalA.IA_DestroyPortalA"))
  ;[0 0.8583 1] PortalA
  (:`Triggered`
    (bind _outactors (`GameplayStatics.GetAllActorsOfClass` "/PortalGame/Blueprints/Portal/BP_Portal.BP_Portal_C"))
    (for _array_element _outactors
      (if (and (not (`Portal.bIsExitPortal` _array_element)) (`self.IsLocalPlayerController`))
        (`/Engine/EditorBlueprintResources/ActorMacros.Switch Has Authority`
          (:`Authority`
            (bind _returnvalue (`Pawn.IsLocallyControlled` (`Actor.Instigator` _array_element)))
            (if _returnvalue
              (`self.K2_DestroyActor` _array_element)))
          (:`Remote`
            (if _returnvalue
              (`self.ServerDestroyPortal` _array_element))))))))

(event `EnhancedInput|/PortalGame/Input/Actions/IA_PortalB`
  (params (ActionValue :type Boolean) (ElapsedSeconds :type "Float (double-precision)") (TriggeredSeconds :type "Float (double-precision)") (InputAction :type "InputAction Object Reference" :default "/PortalGame/Input/Actions/IA_PortalB.IA_PortalB"))
  ;[1 0.4177 0.05486] PortalB
  (:`Triggered`
    (`self.SendGameplayEventWithPayload` (struct :`TagName` "Event.PortalB"))))

(event `EnhancedInput|/PortalGame/Input/Actions/IA_DestroyPortalB`
  (params (ActionValue :type Boolean) (ElapsedSeconds :type "Float (double-precision)") (TriggeredSeconds :type "Float (double-precision)") (InputAction :type "InputAction Object Reference" :default "/PortalGame/Input/Actions/IA_DestroyPortalB.IA_DestroyPortalB"))
  ;[1 0.4177 0.05486] PortalB
  (:`Triggered`
    (bind _outactors (`GameplayStatics.GetAllActorsOfClass` "/PortalGame/Blueprints/Portal/BP_Portal.BP_Portal_C"))
    (for _array_element _outactors
      (if (and (`Portal.bIsExitPortal` _array_element) (`self.IsLocalPlayerController`))
        (`/Engine/EditorBlueprintResources/ActorMacros.Switch Has Authority`
          (:`Authority`
            (bind _returnvalue (`Pawn.IsLocallyControlled` (`Actor.Instigator` _array_element)))
            (if _returnvalue
              (`self.K2_DestroyActor` _array_element)))
          (:`Remote`
            (if _returnvalue
              (`self.ServerDestroyPortal` _array_element))))))))

(fn `UserConstructionScript`)